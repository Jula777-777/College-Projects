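; Wizard character Blueprint that periodically casts a fireball on its own.
; Tick feeds a random 5 to 15 second Delay that triggers the Attack event.
; Attack plays the attack animation, spawns a Fireball actor at the PointLight's transform partway through, then returns to the looping idle animation.
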(event Custom|Attack
  (Components|Animation|PlayAnimation (Variables|SkeletalMeshActor|GetSkeletalMeshComponent) "/Game/BattleWizardPolyart/Animations/Attack01Anim.Attack01Anim" false)
  (Utilities|FlowControl|Delay 0.5)
  (Game|SpawnActorfromClass "/Game/Fireball.Fireball_C" (Transformation|GetWorldTransform (Variables|Default|GetPointLight)) "Undefined" 0 0)
  (Utilities|FlowControl|Delay 0.833333)
  (Components|Animation|PlayAnimation (Variables|SkeletalMeshActor|GetSkeletalMeshComponent) "/Game/BattleWizardPolyart/Animations/Idle01Anim.Idle01Anim" true))

(event EventBeginPlay)

(event Collision|EventActorBeginOverlap
  (params (OtherActor :type Actor%20Object%20Reference)))

(event EventTick
  (params (DeltaSeconds :type Float%20%28single-precision%29))
  (Utilities|FlowControl|Delay (Math|Random|RandomFloatinRange 5.0 15.0))
  (CallFunction|Attack))

(fn ConstructionScript)