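; CoinsBP is a spinning coin pickup that disappears with a collect sound when something overlaps it.
; A Spin timeline starts on BeginPlay and adds its rotation factor to the actor's initial yaw.
; The first PickupCol overlap passes a DoOnce, then hides the mesh, disables its collision and plays the sound.
; It does not filter the overlapping actor, update any score or destroy itself.
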(event OnComponentBeginOverlap(PickupCol)
  (params (OverlappedComponent :type Primitive%20Component%20Object%20Reference) (OtherActor :type Actor%20Object%20Reference) (OtherComp :type Primitive%20Component%20Object%20Reference) (OtherBodyIndex :type Integer) (bFromSweep :type Boolean) (SweepResult :type Hit%20Result%20Structure%20%28by%20ref%29))
  (Utilities|FlowControl|DoOnce false
    (:Completed
      (Development|SetHiddeninGame (Variables|Default|GetPickupMesh) true false)
      (Collision|SetCollisionEnabled (Variables|Default|GetPickupMesh) "NoCollision")
      (Audio|PlaySoundatLocation "/Game/Coins/Game-coin-collect-620.Game-coin-collect-620" (Transformation|GetWorldLocation (Variables|Default|GetPickupCol)) "0, 0, 0" 1.0 1.0 0.0 0 0 0))))

(event EventBeginPlay
  (Variables|Default|SetInitial%20Rotation (Transformation|GetActorRotation))
  (bind _rotation_factor (Timeline|Spin Play)
    (:Update
      (Transformation|SetActorRotation (Math|Rotator|MakeRotator 0.0 0.0 (+ _rotation_factor (.yaw (Variables|Default|GetInitial%20Rotation))))))))

(fn ConstructionScript)